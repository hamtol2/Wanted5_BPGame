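; BP_Cow is a toy cow gimmick that launches the player straight up on contact.
; BeginPlay creates a dynamic material instance on the mesh and sets its BodyColor to the origin color.
; The Box trigger switches BodyColor to the collide color for any overlapping actor and restores it when an overlap ends.
; Characters tagged Player also receive an upward velocity-change impulse through CharacterMovement, scaled by PushPower.
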(event OnComponentBeginOverlap(Box)
  (params (OverlappedComponent :type Primitive%20Component%20Object%20Reference) (OtherActor :type Actor%20Object%20Reference) (OtherComp :type Primitive%20Component%20Object%20Reference) (OtherBodyIndex :type Integer) (bFromSweep :type Boolean) (SweepResult :type Hit%20Result%20Structure%20%28by%20ref%29))
  (Rendering|Material|SetVectorParameterValue (Variables|Default|GetMaterialInstance) "BodyColor" (Variables|Color|GetCollideColor) :!class /Script/Engine.MaterialInstanceDynamic)
  (if (Actor|ActorHasTag OtherActor "Player") ; If 구문 역할
    (bind _ascharacter (Utilities|Casting|CastToCharacter OtherActor))
    (Physics|AddImpulse (Variables|/Script/Engine.Character|GetCharacterMovement _ascharacter) (* (Math|Vector|MakeVector 0.0 0.0 1.0) (Variables|Default|GetPushPower)) true)))

(event OnComponentEndOverlap(Box)
  (params (OverlappedComponent :type Primitive%20Component%20Object%20Reference) (OtherActor :type Actor%20Object%20Reference) (OtherComp :type Primitive%20Component%20Object%20Reference) (OtherBodyIndex :type Integer))
  (Rendering|Material|SetVectorParameterValue (Variables|Default|GetMaterialInstance) "BodyColor" (Variables|Color|GetOriginColor) :!class /Script/Engine.MaterialInstanceDynamic))

(event EventBeginPlay
  (bind _returnvalue (Rendering|Material|CreateDynamicMaterialInstance (Variables|Default|GetStaticMesh) 0 "/Game/Toycow/M_ToyCow.M_ToyCow" "None" :!class /Script/Engine.PrimitiveComponent))
  (bind _output_get (Variables|Default|SetMaterialInstance _returnvalue))
  (Rendering|Material|SetVectorParameterValue _output_get "BodyColor" (Variables|Color|GetOriginColor) :!class /Script/Engine.MaterialInstanceDynamic))

(fn ConstructionScript)