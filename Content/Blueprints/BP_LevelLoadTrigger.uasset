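; BP_LevelLoadTrigger is a trigger actor that streams in a level when an actor tagged Player overlaps it.
; The overlap loads the TargetLevel soft reference as a blocking load and makes it visible immediately.
; An unconnected chain that prints a debug message, waits, then sets the streaming level visible never runs.
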(event EventBeginPlay)

(event Collision|EventActorBeginOverlap
  (params (OtherActor :type Actor%20Object%20Reference))
  (if (Actor|ActorHasTag OtherActor "Player")
    (Class|GameplayStatics|LoadStreamLevelbySoftObjectPtr (Variables|Default|GetTargetLevel) true true)))

(fn ConstructionScript)