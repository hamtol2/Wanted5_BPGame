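; BP_MonsterStat is a component that tracks a monster's current health.
; On BeginPlay it sets CurrentHp to the MaxHp in the MonsterStat of MonsterData, if that data is valid.
; ReceiveDamage subtracts damage, clamps health at zero and broadcasts the OnHpZero event whenever the result is zero.
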(event Custom|ReceiveDamage
  (params (Damage :type Float%20%28double-precision%29))
  ;[0.15 0.1199 0.08671 0.5] 대미지 처리(체력 깎기) 및 HP Zero 이벤트 호출(발행)
  (bind _output_get (Variables|Default|SetCurrentHp (Math|Float|Max(Float) (- (Variables|Default|GetCurrentHp) Damage) 0.0)))
  (if (== _output_get 0.0)
    (Default|CallOnHpZero)))

(event EventBeginPlay
  ;[0.15 0.1294 0.05555 0.5] 시작할 때 최대 체력으로 설정
  (bind _monsterdata (Variables|Default|GetMonsterData)
    (:then
      (Variables|Default|SetCurrentHp (.maxhp (Variables|/Game/Blueprints/Game/Monster/Data/BP_MonsterData.BP_MonsterData_C|GetMonsterStat _monsterdata))))
    (:else)))