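; BP_MainCharacter is the player character, handling movement, camera look and weapon attacks via Enhanced Input.
; A CharacterState gates movement and attacks to Locomotion; attacking requires a valid weapon, plays an attack montage and switches to Attack until OnAttackEnd restores Locomotion.
; Collected weapons attach to the WeaponPosition mesh socket, and bound attack-check start/end events are forwarded to the weapon.
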(event Custom|OnAttack
  ;[0.15 0.062 0.1054 0.5] 공격 시작 처리
  (Utilities|IsValid (Variables|Default|GetWeapon)
    (:Is%20Valid
      ;;[0.15 0.01447 0.007303 0.5] 기본 상태인지 확인
      (switch Utilities|FlowControl|Switch|SwitchonE_CharacterState (Variables|Default|GetCharacterState)
        (:NewEnumerator0
          (Animation|Montage|MontagePlay (Components|SkeletalMesh|GetAnimInstance (Variables|Character|GetMesh)) "/Game/Blueprints/Game/Animation/AM_Attack.AM_Attack" 1.0 "MontageLength" 0.0 true)
          (Variables|Default|SetCharacterState "NewEnumerator1"))))))

(event Custom|OnAttackEnd
  ;[0.15 0.08548 0.04728 0.5] 공격 종료 처리
  (Variables|Default|SetCharacterState "NewEnumerator0"))

(event Custom|OnWeaponCollected
  (params (Weapon :type BP%20Weapon%20Object%20Reference))
  ;[0.1006 0.15 0.099 0.5] 무기 획득 처리
  (bind _output_get (Variables|Default|SetWeapon Weapon))
  (Transformation|AttachComponentToComponent _output_get (Variables|Character|GetMesh) "WeaponPosition" "SnapToTarget" "SnapToTarget" "SnapToTarget" true)
  ;[0.15 0.08647 0.05819 0.5] 이벤트 구독 처리
  (EventDispatchers|BindEventtoAttackCheckStart (delegate Custom|OnAttackCheckStart)) ; 이 이벤트에 다른 이벤트를 연결
  (EventDispatchers|BindEventtoAttackCheckEnd (delegate Custom|OnAttackCheckEnd)))

(event Custom|OnAttackCheckStart
  ;[0.15 0.08647 0.05819 0.5] 이벤트 구독 처리
  (Default|OnAttackCheckStart (Variables|Default|GetWeapon)))

(event Custom|OnAttackCheckEnd
  ;[0.15 0.08647 0.05819 0.5] 이벤트 구독 처리
  (Default|OnAttackCheckEnd (Variables|Default|GetWeapon)))

(event Input|EnhancedActionEvents|EnhancedInputActionIA_Move
  (params (ActionValue :type Vector%202D%20Structure) (ElapsedSeconds :type Float%20%28double-precision%29) (TriggeredSeconds :type Float%20%28double-precision%29) (InputAction :type Input%20Action%20Object%20Reference :default "/Game/Blueprints/Input/IA_Move.IA_Move"))
  (bind _returnvalue (Pawn|GetControlRotation :!class /Script/Engine.Pawn))
  ;[0.0225 0.15 0.01676 0.5] 이동
  (switch Utilities|FlowControl|Switch|SwitchonE_CharacterState (Variables|Default|GetCharacterState)
    (:NewEnumerator0
      (Pawn|Input|AddMovementInput (+ (* (Math|Vector|GetRightVector (Math|Rotator|MakeRotator 0.0 0.0 (.yaw _returnvalue))) (.x ActionValue)) (* (Math|Vector|GetForwardVector (Math|Rotator|MakeRotator 0.0 0.0 (.yaw _returnvalue))) (.y ActionValue))) 1.0 false))))

(event Input|EnhancedActionEvents|EnhancedInputActionIA_Look
  (params (ActionValue :type Vector%202D%20Structure) (ElapsedSeconds :type Float%20%28double-precision%29) (TriggeredSeconds :type Float%20%28double-precision%29) (InputAction :type Input%20Action%20Object%20Reference :default "/Game/Blueprints/Input/IA_Look.IA_Look"))
  ;[0.15 0.123 0.009736 0.5] 카메라 회전
  (Pawn|Input|AddControllerYawInput (.x ActionValue))
  (Pawn|Input|AddControllerPitchInput (* (.y ActionValue) -1.0)))

(event Input|EnhancedActionEvents|EnhancedInputActionIA_Attack
  (params (ActionValue :type Boolean) (ElapsedSeconds :type Float%20%28double-precision%29) (TriggeredSeconds :type Float%20%28double-precision%29) (InputAction :type Input%20Action%20Object%20Reference :default "/Game/Blueprints/Input/IA_Attack.IA_Attack"))
  ;[0.15 0.08727 0.03053 0.5] 공격 입력 처리 -> 공격 이벤트 실행
  (:Started
    (CallFunction|OnAttack)))

(fn ConstructionScript)