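; Bear monster character that spots the player, chases and dies, with behavior driven by an AI Blackboard.
; Pawn sensing sets the target and Chase state; SetState syncs the Blackboard and adjusts walk speed from stat data, with Dead as terminal.
; Damage feeds the MonsterStat component and flashes a dynamic material parameter through a timeline.
; Zero HP disables collision, plays a death montage, stops AI logic and destroys the actor after a delay.
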(event OnSeePawn(PawnSensing)
  (params (Pawn :type Pawn%20Object%20Reference))
  ;[0.15 0.1259 0.03749 0.5] 플레이어 시야 감지
  (switch Utilities|FlowControl|Switch|SwitchonEBearState (Variables|Default|GetBearState)
    (:NewEnumerator0
      (if (Actor|ActorHasTag Pawn "Player")
        (AI|Components|Blackboard|SetValueasObject (Variables|/Script/AIModule.AIController|GetBlackboard (AI|GetAIController self)) (Variables|Default|GetTargetPlayerKey) Pawn)
        (CallFunction|SetState "NewEnumerator1")))))

(event Custom|PlayDamageEffect
  ;[0.15 0.134 0.04552 0.5] 피격 효과 재생(머티리얼 활용)
  (bind _alpha (Timeline|DamageEffect PlayFromStart)
    (:Update
      (bind _materialinstance (Variables|Default|GetMaterialInstance)
        (:then
          (Rendering|Material|SetScalarParameterValue _materialinstance "DamageFactor" _alpha :!class /Script/Engine.MaterialInstanceDynamic))
        (:else)))
    (:Finished
      (bind _materialinstance_2 (Variables|Default|GetMaterialInstance)
        (:then
          (Rendering|Material|SetScalarParameterValue _materialinstance_2 "DamageFactor" 0.0 :!class /Script/Engine.MaterialInstanceDynamic))
        (:else)))))

(event Custom|MonsterDied
  (bind _self self)
  (bind _returnvalue (AI|GetAIController _self))
  (bind _braincomponent (Variables|/Script/AIModule.AIController|GetBrainComponent _returnvalue))
  ;[0.15 0.15 0.15 0.5] 죽음 이벤트 등록 및 처리
  (Collision|SetActorEnableCollision false) ; 액터의 모든 콜리전 끄기
  (Animation|PlayAnimMontage "/Game/Blueprints/Game/Monster/Animation/AM_MonsterDead.AM_MonsterDead" 1.0 "None") ; 죽는 모션 재생
  ;;[0.15 0.007311 0.03617 0.5] AI 중지 처리
  (AI|Logic|StopLogic _braincomponent "")
  (Class|NavMovementInterface|StopMovementKeepPathing(Message) _braincomponent)
  (CallFunction|SetState "NewEnumerator3")
  (Utilities|FlowControl|Delay 2.0)
  (Actor|DestroyActor))

(event Collision|EventActorBeginOverlap
  (params (OtherActor :type Actor%20Object%20Reference)))

(event Game|Damage|EventAnyDamage
  (params (Damage :type Float%20%28single-precision%29) (DamageType :type Damage%20Type%20Object%20Reference) (InstigatedBy :type Controller%20Object%20Reference) (DamageCauser :type Actor%20Object%20Reference))
  ;[0.06209 0.15 0.05404 0.5] 몬스터 대미지 처리
  (CallFunction|PlayDamageEffect)
  (Default|ReceiveDamage (Variables|Default|GetMonsterStat) Damage))

(event EventBeginPlay
  ;[0.15 0.15 0.15 0.5] 머티리얼 인스턴스 생성(피격 효과를 위해)
  (bind _returnvalue (Rendering|Material|CreateDynamicMaterialInstance (Variables|Character|GetMesh) 0 "/Game/InfinityBladeAdversaries/Enemy/Enemy_Bear/Materials/M_Bear_Stone_Inst.M_Bear_Stone_Inst" "None" :!class /Script/Engine.PrimitiveComponent))
  (Variables|Default|SetMaterialInstance _returnvalue)
  ;[0.15 0.15 0.15 0.5] 죽음 이벤트 등록 및 처리
  (EventDispatchers|BindEventtoOnHpZero (Variables|Default|GetMonsterStat) (delegate Custom|MonsterDied)))

(fn ConstructionScript)

(fn SetState
  (params (NewState :type EBearState%20Enum :default "NewEnumerator0"))
  (bind _charactermovement (Variables|Character|GetCharacterMovement))
  (bind _monsterstat (Variables|Default|GetMonsterStat))
  (bind _monsterdata (Variables|/Game/Blueprints/Game/Component/BP_MonsterStat.BP_MonsterStat_C|GetMonsterData _monsterstat))
  (bind _monsterstat_2 (Variables|/Game/Blueprints/Game/Monster/Data/BP_MonsterData.BP_MonsterData_C|GetMonsterStat _monsterdata))
  (if (Utilities|Enum|NotEqual(Enum) (Variables|Default|GetBearState) "NewEnumerator3")
    (bind _output_get (Variables|Default|SetBearState NewState))
    (AI|Components|Blackboard|SetValueasEnum (Variables|/Script/AIModule.AIController|GetBlackboard (AI|GetAIController self)) (Variables|Default|GetStateKey) _output_get)
    (switch Utilities|FlowControl|Switch|SwitchonEBearState (Variables|Default|GetBearState)
      (:NewEnumerator0
        (Variables|/Script/Engine.CharacterMovementComponent|SetMaxWalkSpeed _charactermovement (.walkspeed _monsterstat_2)))
      (:NewEnumerator1
        (Variables|/Script/Engine.CharacterMovementComponent|SetMaxWalkSpeed _charactermovement (.chasespeed _monsterstat_2)))
      (:NewEnumerator2
        (Variables|/Script/Engine.CharacterMovementComponent|SetMaxWalkSpeed _charactermovement 0.0 :!label _label))
      (:NewEnumerator3
        (goto _label)))))